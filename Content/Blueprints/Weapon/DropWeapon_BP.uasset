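; DropWeapon_BP is a dropped weapon actor that lies in the world as a physics object and can be highlighted, apparently for pickup.
; The construction script sets WeaponMesh from the static mesh in WeaponData, and BeginPlay turns on physics simulation.
; HighLight and EndHighLight apply and clear an overlay material on the mesh, leaving its base materials untouched.
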(event EventBeginPlay
  (Physics|SetSimulatePhysics (Variables|Default|GetWeaponMesh) true))

(event Collision|EventActorBeginOverlap
  (params (OtherActor :type Actor%20Object%20Reference)))

(event EventTick
  (params (DeltaSeconds :type Float%20%28single-precision%29)))

(event EventEndHighLight
  (Rendering|Material|SetOverlayMaterial (Variables|Default|GetWeaponMesh) 0 :!class /Script/Engine.MeshComponent))

(event EventHighLight
  (Rendering|Material|SetOverlayMaterial (Variables|Default|GetWeaponMesh) "/Game/items/PickUpHignLight.PickUpHignLight" :!class /Script/Engine.MeshComponent))

(fn ConstructionScript
  (Components|StaticMesh|SetStaticMesh (Variables|Default|GetWeaponMesh) (Variables|/Game/items/Weapon_DataAssets.Weapon_DataAssets_C|GetStaticMesh (Variables|Default|GetWeaponData))))