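; TimeSwitchComponent is a gameplay component for switching between timeframes and deciding whether an object is hidden in the current one.
; The TimeSwitch event flips the CurrentTime boolean and prints the new value.
; A separate CheckTimeframe event reports the object as hidden when both IsInThePast and CurrentTime are false, otherwise unhidden.
; Both events only print strings; neither changes actual visibility or calls the other.
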(event Custom|TimeSwitch
  ;[0.4667 0.2339 1] TimeSwitch Input
  (bind _output_get (Variables|Default|SetcurrentTime (== (Variables|Default|GetcurrentTime) false)))
  (Development|PrintString (Utilities|String|ToString(Boolean) _output_get)))

(event Custom|CheckTimeframe
  ;[0.1703 0.2932 1] Hide depending on Timeframe
  (if (Math|Boolean|NORBoolean (Variables|Default|GetisInThePast) (Variables|Default|GetcurrentTime))
    (Development|PrintString "Object Is Hidden")
    (else
      (Development|PrintString "Object Is Unhidden"))))