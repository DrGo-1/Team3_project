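; Actor component that tracks an entity's health, starting CurrentHealth at BaseHealth on BeginPlay.
; The ModifyHealthInstant event routes an amount to HealthIncrease or HealthDecrease based on a healing flag.
; Those functions clamp the result between zero and BaseHealth and print the new value to screen.
; No death handling or change notification is present, and an empty CustomEvent is left unused.
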(event Custom|ModifyHealthInstant
  (params (healthModifier :type Integer) (isHealing :type Boolean))
  ;[1 0.04688 0.04688] Modify Health
  (if isHealing
    (CallFunction|HealthIncrease healthModifier)
    (else
      (CallFunction|HealthDecrease healthModifier))))

(event Custom|CustomEvent
  ;[1 0.04688 0.04688] Modify Health
)

(event EventBeginPlay
  (Variables|Default|SetcurrentHealth (Variables|Default|GetbaseHealth)))

(fn HealthIncrease
  (params (healthInput :type Integer))
  (bind _output_get (Variables|Default|SetcurrentHealth (Math|Integer|Min(Integer) (+ healthInput (Variables|Default|GetcurrentHealth)) (Variables|Default|GetbaseHealth))))
  (Development|PrintString (Utilities|String|ToString(Integer) _output_get)))

(fn HealthDecrease
  (params (healthInput :type Integer))
  (bind _output_get (Variables|Default|SetcurrentHealth (Math|Integer|Max(Integer) (- (Variables|Default|GetcurrentHealth) healthInput))))
  (Development|PrintString (Utilities|String|ToString(Integer) _output_get)))