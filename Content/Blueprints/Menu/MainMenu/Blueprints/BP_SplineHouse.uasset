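; Main menu spline actor that lines both sides of its spline with random houses from the Houses array.
; The construction script spawns two rows, one house per side at each spline point, through GetSplineData's randomized side offset and quarter-turn yaw.
; A downward visibility trace snaps each house to the ground, slightly sunk, falling back to the computed point on a miss.
; Only the first row applies the random rotation.
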(event EventBeginPlay)

(event Collision|EventActorBeginOverlap
  (params (OtherActor :type Actor%20Object%20Reference)))

(event EventTick
  (params (DeltaSeconds :type Float%20%28single-precision%29)))

(fn ConstructionScript
  (CallFunction|MyConstructionScript))

(fn MyConstructionScript
  ;[1 1 1] First row
  (Utilities|FlowControl|Sequence
    (:then_0
      (for _index (range 0 (- (Spline|GetNumberOfSplinePoints (Variables|Default|GetSpline)) 1))
        (LocalVariables|SetSpawnLocation (.SpawnLocation (CallFunction|GetSplineData _index true)))
        (LocalVariables|SetSpawnRotation (.SpawnRotation (CallFunction|GetSplineData _index true)))
        (LocalVariables|SetSpawningHouse (.SpawnHouse (CallFunction|GetSplineData _index true)))
        (bind (_outhit _returnvalue) (Collision|LineTraceByChannel (+ "0.000000,0.000000,500.000000" (LocalVariables|GetSpawnLocation)) (+ (LocalVariables|GetSpawnLocation) "0.000000,0.000000,-2000.000000") "TraceTypeQuery1" false 0 "None"))
        (LocalVariables|SetUseTrace _returnvalue)
        (Game|SpawnActorfromClass (LocalVariables|GetSpawningHouse) (Math|Transform|MakeTransform (+ (Math|Vector|SelectVector (.Location (Collision|BreakHitResult _outhit)) (LocalVariables|GetSpawnLocation) (LocalVariables|GetUseTrace)) "0.000000,0.000000,-50.000000") (LocalVariables|GetSpawnRotation) "1.000000,1.000000,1.000000") "Undefined" "MultiplyWithRoot" 0 (Game|GetInstigator))))
    (:then_1
      ;[1 1 1] Second row
      (for _index_2 (range 0 (- (Spline|GetNumberOfSplinePoints (Variables|Default|GetSpline)) 1))
        (LocalVariables|SetSpawnLocation (.SpawnLocation (CallFunction|GetSplineData _index_2 false)))
        (LocalVariables|SetSpawnRotation (.SpawnRotation (CallFunction|GetSplineData _index_2 false)))
        (LocalVariables|SetSpawningHouse (.SpawnHouse (CallFunction|GetSplineData _index_2 false)))
        (bind (_outhit_2 _returnvalue_2) (Collision|LineTraceByChannel (+ "0.000000,0.000000,500.000000" (LocalVariables|GetSpawnLocation)) (+ (LocalVariables|GetSpawnLocation) "0.000000,0.000000,-2000.000000") "TraceTypeQuery1" false 0 "None"))
        (LocalVariables|SetUseTrace _returnvalue_2)
        (Game|SpawnActorfromClass (LocalVariables|GetSpawningHouse) (Math|Transform|MakeTransform (+ (Math|Vector|SelectVector (.Location (Collision|BreakHitResult _outhit_2)) (LocalVariables|GetSpawnLocation) (LocalVariables|GetUseTrace)) "0.000000,0.000000,-50.000000") "0, 0, 0" "1.000000,1.000000,1.000000") "Undefined" "MultiplyWithRoot" 0 (Game|GetInstigator))))))

(fn GetSplineData
  (params (PointIndex :type Integer) (Right :type Boolean))
  (bind _spline (Variables|Default|GetSpline))
  (bind _houses (Variables|Default|GetHouses))
  (bind _returnvalue (Spline|GetSplinePointAt _spline PointIndex "World"))
  (bind (_position _rotation) (Utilities|Struct|BreakSplinePoint _returnvalue))
  (bind (_roll _pitch) (Math|Rotator|BreakRotator _rotation))
  (return (+ (+ (Transformation|GetActorLocation) _position) (* (Math|Vector|GetRightVector _rotation) (* (Math|Random|RandomFloatinRange 8e+02 1.3e+03) (Math|Float|SelectFloat 1.0 -1.0 Right)))) (Math|Rotator|MakeRotator _roll _pitch (* 9e+01 (Math|Random|RandomIntegerinRange 0 3))) (Utilities|Array|Get(acopy) _houses (Math|Random|RandomIntegerinRange 0 (Utilities|Array|LastIndex _houses)))))