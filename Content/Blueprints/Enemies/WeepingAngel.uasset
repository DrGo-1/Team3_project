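; Weeping Angel enemy Blueprint that continually hunts the first player character.
; On BeginPlay it casts player 0 to Player_BP, stores the reference and starts the AiMoveTo event, printing debug messages along the way.
; AiMoveTo moves the angel toward the player, then calls itself again after a short delay on either success or failure.
; The graph contains no line-of-sight or freeze-when-watched logic.
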(event Custom|AiMoveTo
  ;[1 0.3955 0.4154] player variable as target for moving, printing to see failure points a delay and a loop
  (bind _movementresult (AI|AIMoveTo self "0, 0, 0" (Variables|Default|GetAs%20Player%20BP) 5.0 false)
    (:OnSuccess
      _)
    (:OnFail
      _))
  (Development|PrintString (Utilities|String|EnumtoString _movementresult))
  (Utilities|FlowControl|Delay 0.2)
  (CallFunction|AiMoveto))

(event EventBeginPlay
  ;[0.4048 0.9602 1] Get player character 0, as 0 is the first number. Cast to get a correct bp for our variable that the angel will hunt. then activate the hunt event.
  (bind _asplayer_bp (Utilities|Casting|CastToPlayer_BP (Game|GetPlayerCharacter 0))
    (:then
      (Utilities|IsValid _asplayer_bp
        (:Is%20Valid
          (Variables|Default|SetAs%20Player%20BP _asplayer_bp)
          (CallFunction|AiMoveto)
          (Development|PrintString "Beginplay"))
        (:Is%20Not%20Valid
          (Development|PrintString "WeepingIsValidFail"))))
    (:CastFailed
      (Development|PrintString "failed cast"))))

(fn ConstructionScript)