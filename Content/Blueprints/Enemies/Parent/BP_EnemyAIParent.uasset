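; Parent AI controller for enemies that runs the enemy behavior tree and feeds perception results into its blackboard.
; Perception updates are split by sense: sight sets or clears the Player key, and hearing shifts recent noise locations through two ImportantLocation keys.
; Losing sight stores the last seen location and, after a short delay, requests a prediction event, whose predicted location becomes ImportantLocation1, with a debug sphere trace.
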(event EventBeginPlay
  (bind _returnvalue (AI|RunBehaviorTree "/Game/Blueprints/Enemies/Parent/BehaviorTreeBlackBoard/BehaviorTree_EnemyParent.BehaviorTree_EnemyParent"))
  (Development|PrintString (Utilities|String|Append "RunBehavior" (Utilities|String|ToString(Boolean) _returnvalue)) true true "(R=0.000000,G=0.660000,B=1.000000,A=1.000000)" 5.0))

(event OnTargetPerceptionUpdated(AIPerception)
  (params (Actor :type Actor%20Object%20Reference) (Stimulus :type AI%20Stimulus%20Structure))
  ;[1 1 1] Set variables from stimuli and actor
  (CallFunction|GetSense Actor Stimulus)
  ;[1 1 1] Switch on sense type
  (switch string (Variables|Default|GetStimulusSense)
    (:AISense_Sight
      (CallFunction|SightSense))
    (:AISense_Hearing
      (CallFunction|HearingSense))
    (:AISense_Prediction
      (CallFunction|PredictionSense))))

(event Custom|GetPrediction
  (params (PredictedActor :type Actor%20Object%20Reference))
  (Utilities|FlowControl|Delay 0.1)
  (Class|AISensePrediction|RequestControllerPredictionEvent self PredictedActor 2.0))

(fn ConstructionScript)

(fn GetSense
  (params (SeenActor :type Actor%20Object%20Reference) (AIStimulus :type AI%20Stimulus%20Structure%20%28by%20ref%29))
  (bind (_age _expirationage _strength _stimuluslocation _receiverlocation _tag _bsuccessfullysensed) (Utilities|Struct|BreakAIStimulus AIStimulus))
  (Variables|Default|SetSensedActor SeenActor)
  (bind _returnvalue (Class|AIPerceptionSystem|GetSenseClassforStimulus AIStimulus))
  (Variables|Default|SetStimulusSense (Utilities|GetClassDisplayName _returnvalue))
  (Variables|Default|SetStimulus%20Location _stimuluslocation)
  (Variables|Default|SetStimulusTag _tag)
  (Variables|Default|SetStimulus%20Successfully%20Sensed _bsuccessfullysensed))

(fn SightSense
  ;[0.7094 0.2993 1] Switch between seen and not seen
  (if (Variables|Default|GetStimulus%20Successfully%20Sensed)
    ;[1 0.228 0.2678] Sight
    (bind _asplayer_bp (Utilities|Casting|CastToPlayer_BP (Variables|Default|GetSensedActor))
      (:then
        (AI|Components|Blackboard|SetValueasObject (AI|GetBlackboard 0) (Utilities|Name|MakeLiteralName "Player") _asplayer_bp)
        (Development|PrintString "SightApplied"))
      (:CastFailed
        (Development|PrintString "SeenCastFail")))
    (else
      ;[0.75 1 0.5] Unsuccessful Sight
      (Utilities|Casting|CastToPlayer_BP (Variables|Default|GetSensedActor)
        (:then
          (AI|Components|Blackboard|SetValueasVector (AI|GetBlackboard 0) (Utilities|Name|MakeLiteralName "ImportantLocation2") (Variables|Default|GetStimulus%20Location))
          (CallFunction|GetPrediction (Variables|Default|GetSensedActor))
          (AI|Components|Blackboard|ClearValue (AI|GetBlackboard 0) (Utilities|Name|MakeLiteralName "Player"))
          (Development|PrintString "SightRemoved"))
        (:CastFailed
          (Development|PrintString "SeenCastFail"))))))

(fn PredictionSense
  (bind _stimulus_location (Variables|Default|GetStimulus%20Location))
  ;[1 0.295 0.9511] Predicted stimulus from a request: most likely sight
  (AI|Components|Blackboard|SetValueasVector (AI|GetBlackboard 0) (Utilities|Name|MakeLiteralName "ImportantLocation1") _stimulus_location)
  (Collision|MultiSphereTraceByChannel _stimulus_location _stimulus_location 2e+02 "TraceTypeQuery1" false 0 "ForDuration"))

(fn HearingSense
  (bind _returnvalue (AI|GetBlackboard 0))
  ;[1 0.7443 0.3727] Successful Hearing
  (if (Variables|Default|GetStimulus%20Successfully%20Sensed)
    (Utilities|Casting|CastToPlayer_BP (Variables|Default|GetSensedActor)
      (:then
        (AI|Components|Blackboard|SetValueasVector _returnvalue (Utilities|Name|MakeLiteralName "ImportantLocation2") (AI|Components|Blackboard|GetValueasVector _returnvalue (Utilities|Name|MakeLiteralName "ImportantLocation1")))
        (AI|Components|Blackboard|SetValueasVector (AI|GetBlackboard 0) (Utilities|Name|MakeLiteralName "ImportantLocation1") (Variables|Default|GetStimulus%20Location))
        (Development|PrintString "HearingApplied"))
      (:CastFailed
        (Development|PrintString "SeenCastFail")))))