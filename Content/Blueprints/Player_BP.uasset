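; Player Blueprint providing first-person movement, look controls and a Tab-triggered "time switch".
; BeginPlay adds the FPS_Input Enhanced Input mapping context, whose actions drive movement along the actor's forward and right vectors plus controller yaw and pitch.
; TimeSwitch uses a counter as a toggle, teleporting the player back and forth by a fixed world-space Y offset, which suggests two parallel copies of the level.
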(event EventBeginPlay
  (bind _returnvalue (Game|GetPlayerController 0))
  (bind _returnvalue_2 (PlayerController|LocalPlayerSubsystems|GetEnhancedInputLocalPlayerSubsystem _returnvalue))
  (Utilities|IsValid _returnvalue_2
    (:Is%20Valid
      (Input|AddMappingContext _returnvalue_2 "/Game/Blueprints/FPS_Input.FPS_Input" 0 "(bIgnoreAllPressedKeysUntilRelease=True,bForceImmediately=False,bNotifyUserSettings=False)"))))

(event Collision|EventActorBeginOverlap
  (params (OtherActor :type Actor%20Object%20Reference)))

(event EventTick
  (params (DeltaSeconds :type Float%20%28single-precision%29)))

(event Custom|TimeSwitch
  ;[1 1 1] TimeSwitch（set the moveing distant with that yellow box)
  (if (> (Variables|Default|GetTimeSwith) 0)
    (Variables|Default|SetTimeSwith (- (Variables|Default|GetTimeSwith) 1))
    (Transformation|SetActorLocation (+ (Transformation|GetActorLocation) "0.000000,-500.000000,0.000000") false false)
    (else
      (Variables|Default|SetTimeSwith (- 0 -1))
      (Transformation|SetActorLocation (+ (Transformation|GetActorLocation) "0.000000,500.000000,0.000000") false false))))

(event Input|EnhancedActionEvents|EnhancedInputActionPlayer_Move
  (params (ActionValue :type Vector%202D%20Structure) (ElapsedSeconds :type Float%20%28double-precision%29) (TriggeredSeconds :type Float%20%28double-precision%29) (InputAction :type Input%20Action%20Object%20Reference :default "/Game/Blueprints/Player_Move.Player_Move"))
  (bind (_x _y) (Math|Vector2D|BreakVector2D ActionValue))
  ;[1 1 1] Move
  (Pawn|Input|AddMovementInput (Transformation|GetActorRightVector) _x false)
  (Pawn|Input|AddMovementInput (Transformation|GetActorForwardVector) _y false))

(event Input|EnhancedActionEvents|EnhancedInputActionPlayer_LookAround
  (params (ActionValue :type Vector%202D%20Structure) (ElapsedSeconds :type Float%20%28double-precision%29) (TriggeredSeconds :type Float%20%28double-precision%29) (InputAction :type Input%20Action%20Object%20Reference :default "/Game/Blueprints/Player_LookAround.Player_LookAround"))
  (bind (_x _y) (Math|Vector2D|BreakVector2D ActionValue))
  ;[1 1 1] LookAround
  (Pawn|Input|AddControllerYawInput _x)
  (Pawn|Input|AddControllerPitchInput _y))

(event Input|KeyboardEvents|Tab
  (params (Key :type Key%20Structure :default "None"))
  ;[1 1 1] TimeSwitch（set the moveing distant with that yellow box)
  (:Pressed
    (CallFunction|TimeSwitch)))

(fn ConstructionScript)